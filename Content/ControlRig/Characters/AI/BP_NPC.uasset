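; An NPC Blueprint that wanders endlessly between random points inside a nav mesh bounds volume.
; On BeginPlay it caches the NavMeshBoundsVolume nearest the world origin and starts the first walk.
; Each walk uses AI MoveTo toward a random point in a box derived from the volume's scale.
; Success draws debug shapes and calls FinishedWalk again, while failure only prints a message and ends the loop.
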(event `Finished Walk`
  (bind _navmesh (`self.NavMesh`))
  (bind _returnvalue (`self.K2_GetActorLocation` _navmesh))
  (bind _returnvalue_2 (* (`self.GetActorRelativeScale3D` _navmesh) (90.0 90.0 10.0)))
  (set `self.NewVar_0` (`KismetMathLibrary.RandomPointInBoundingBox` _returnvalue _returnvalue_2) :!label _label)
  (`|AIMoveTo` self (`self.NewVar_0`) null
    (:`OnSuccess`
      (`KismetSystemLibrary.DrawDebugSphere` (`self.NewVar_0`) 10.0 12 (struct :`R` 1.0 :`B` 0.076571 :`A` 1.0) 100.1)
      (`KismetSystemLibrary.DrawDebugBox` _returnvalue _returnvalue_2 (struct) (struct) 100.0)
      (`KismetSystemLibrary.PrintString` "success")
      (`self.Finished Walk`))
    (:`OnFail`
      (`KismetSystemLibrary.PrintString` "failure"))))

(event `self.ReceiveBeginPlay`
  (bind _outactors (`GameplayStatics.GetAllActorsOfClass` "/Script/NavigationSystem.NavMeshBoundsVolume"))
  (bind _asnav_mesh_bounds_volume (cast `NavMeshBoundsVolume` (`.ReturnValue` (`GameplayStatics.FindNearestActor` (0.0 0.0 0.0) _outactors))))
  (set `self.NavMesh` _asnav_mesh_bounds_volume)
  (goto _label))

(fn `UserConstructionScript`)